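; Health component that tracks an owner's health and handles its death.
; Health starts at the maximum, and damage is subtracted only while damage is allowed, then checked for zero or below.
; On death, flags decide whether to destroy the owner, with an optional death sound and Niagara burst sharing one flag, and whether to reload the current level for player death.
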(event `self.ReceiveBeginPlay`
  (set `self.CurrentHealth` (`self.MaxHealth`)))

(event `Apply Damage`
  (params (DamageTaken :type Integer))
  (if (`self.CanTakeDamage`)
    (bind _output_get (set `self.CurrentHealth` (- (`self.CurrentHealth`) DamageTaken)))
    (`self.Check Dead` _output_get)))

(event `Check Dead`
  (params (Health :type Integer))
  (bind _returnvalue (`Actor.K2_GetActorLocation` (`self.GetOwner`)))
  (if (<= Health 0)
    (`|ExecutionSequence`
      (:`then_0`
        (if (`self.DestroyOnDeath`)
          (if (`self.PlaySoundOnDeath`)
            (`GameplayStatics.PlaySoundAtLocation` "/Game/Sound/MushroomDeath.MushroomDeath" _returnvalue (struct) 2.0 1.0 0.0 null null null null)
            (`NiagaraFunctionLibrary.SpawnSystemAtLocation` "/Game/VFX/CloudBurst/NE_CloudBurst_System.NE_CloudBurst_System" _returnvalue))
          (`Actor.K2_DestroyActor` (`self.GetOwner`))))
      (:`then_1`
        (if (`self.RestartOnPlayerDeath`)
          (bind _returnvalue_2 (`GameplayStatics.GetCurrentLevelName` true))
          (`GameplayStatics.OpenLevel` (`KismetStringLibrary.Conv_StringToName` _returnvalue_2)))))))