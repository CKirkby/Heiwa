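; BP_Boat is a boat actor that bobs up and down along the Z axis.
; BeginPlay waits a random one to two seconds before setting InitialisationComplete, which enables the movement in Tick.
; Each tick adds a sine offset to the current Z, driven by time since creation, BobbingSpeedZ and BobbingDistanceZ.
; The offset accumulates without delta-time scaling, so the motion depends on frame rate.
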(event `self.ReceiveBeginPlay`
  (`KismetSystemLibrary.Delay` (`KismetMathLibrary.RandomFloatInRange` 1.0 2.0))
  (set `self.InitialisationComplete` true))

(event `self.ReceiveTick`
  (params (DeltaSeconds :type "Float (single-precision)"))
  (bind (_returnvalue_x _returnvalue_y _returnvalue_z) (`KismetMathLibrary.BreakVector` (`self.K2_GetActorLocation`)))
  (if (`self.InitialisationComplete`)
    (`self.K2_SetActorLocation` (`KismetMathLibrary.MakeVector` _returnvalue_x _returnvalue_y (+ _returnvalue_z (* (`self.BobbingDistanceZ`) (`KismetMathLibrary.DegSin` (* (`self.GetGameTimeSinceCreation`) (`self.BobbingSpeedZ`)))))))))

(fn `UserConstructionScript`)