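; BP_BoatMoving moves a boat mesh along a spline in an endless loop.
; BeginPlay starts a timeline with a play rate of one over TimeToComplete.
; Each update maps the timeline alpha to spline distance, setting the mesh's world location and rotation with a 90-degree yaw offset.
; When the timeline finishes, ResetSpline replays it from the start, returning the boat to the spline's beginning.
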(event `Reset Spline`
  (bind _spline (`self.Spline`))
  (bind _boatmesh (`self.BoatMesh`))
  (bind (_direction _alpha) (`Timeline|Timeline` :!via `PlayFromStart` :!label _label)
    (:`Update`
      (bind _returnvalue (`KismetMathLibrary.Lerp` 0.0 (`SplineComponent.GetSplineLength` (`self.Spline`)) _alpha))
      (`SceneComponent.K2_SetWorldLocation` _boatmesh (`SplineComponent.GetLocationAtDistanceAlongSpline` _spline _returnvalue "World") false false)
      (`SceneComponent.K2_SetWorldRotation` _boatmesh (`KismetMathLibrary.MakeRotator` (.roll (`SplineComponent.GetRotationAtDistanceAlongSpline` _spline _returnvalue "World")) (.pitch (`SplineComponent.GetRotationAtDistanceAlongSpline` _spline _returnvalue "World")) (+ (.yaw (`SplineComponent.GetRotationAtDistanceAlongSpline` _spline _returnvalue "World")) 90.0)) false false))
    (:`Finished`
      (`self.Reset Spline`))))

(event `self.ReceiveBeginPlay`
  (`TimelineComponent.SetPlayRate` (`self.Timeline`) (/ 1.0 (`self.TimeToComplete`)))
  (goto _label))

(fn `UserConstructionScript`)