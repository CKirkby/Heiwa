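; Base enemy character that wakes when the player approaches and melee-attacks them, using mushroom animation montages.
; It feeds its AI controller's blackboard the player as target, plus inactive, visible and attacking flags driven by detection and attack radius overlaps.
; Attack plays a montage, then after a short delay sphere-traces at AttackPoint to damage the player.
; Incoming damage goes to HealthComponent and plays the alert montage.
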(event `self.ReceiveBeginPlay`
  (`self.SetBlackboardTargetActor`)
  (`self.SetBlackBoardIsInactive` (`self.IsInactive`)))

(event `self.ReceiveTick`
  (params (DeltaSeconds :type "Float (single-precision)"))
  (if true
    _))

(event `self.DetectionRadius.OnComponentBeginOverlap`
  (params (OverlappedComponent :type "PrimitiveComponent Object Reference") (OtherActor :type "Actor Object Reference") (OtherComp :type "PrimitiveComponent Object Reference") (OtherBodyIndex :type Integer) (bFromSweep :type Boolean) (SweepResult :type "HitResult Structure (by ref)"))
  (if (`self.ActorHasTag` OtherActor "Player")
    (set `self.IsInactive` false)
    (`KismetSystemLibrary.Delay` 1.5)
    (`self.SetBlackBoardIsInactive` false)
    (`self.SetBlackboardTargetVisible`)))

(event `self.AttackRadius.OnComponentBeginOverlap`
  (params (OverlappedComponent :type "PrimitiveComponent Object Reference") (OtherActor :type "Actor Object Reference") (OtherComp :type "PrimitiveComponent Object Reference") (OtherBodyIndex :type Integer) (bFromSweep :type Boolean) (SweepResult :type "HitResult Structure (by ref)"))
  (if (`self.ActorHasTag` OtherActor "Player")
    (`self.SetBlackboardIsAttacking` true)))

(event `self.AttackRadius.OnComponentEndOverlap`
  (params (OverlappedComponent :type "PrimitiveComponent Object Reference") (OtherActor :type "Actor Object Reference") (OtherComp :type "PrimitiveComponent Object Reference") (OtherBodyIndex :type Integer))
  (if (`self.ActorHasTag` OtherActor "Player")
    (`self.SetBlackboardIsAttacking` false)))

(event `Attack`
  (bind _returnvalue (`SceneComponent.K2_GetComponentLocation` (`self.AttackPoint`)))
  (`self.PlayAnimMontage` "/Game/Animation/Mushroom/New/Mushroom_Attack_Animation_Montage.Mushroom_Attack_Animation_Montage")
  (`KismetSystemLibrary.Delay` 0.5)
  (bind (_outhit _returnvalue_2) (`KismetSystemLibrary.SphereTraceSingle` _returnvalue _returnvalue 100.0 "TraceTypeQuery1"))
  (if _returnvalue_2
    (bind (_bblockinghit _binitialoverlap _time _distance _location _impactpoint _normal _impactnormal _physmat _hitactor) (`GameplayStatics.BreakHitResult` _outhit))
    (`/Engine/EditorBlueprintResources/StandardMacros.IsValid` _hitactor
      (:`Is Valid`
        (if (`self.ActorHasTag` _hitactor "Player")
          (`GameplayStatics.ApplyDamage` _hitactor 1.0 null self))))))

(event `self.ReceiveAnyDamage`
  (params (Damage :type "Float (single-precision)") (DamageType :type "DamageType Object Reference") (InstigatedBy :type "Controller Object Reference") (DamageCauser :type "Actor Object Reference"))
  (`/Game/Programming/Blueprints/Components/HealthComponent.Apply Damage` (`self.HealthComponent`) (`KismetMathLibrary.FFloor` Damage))
  (`self.PlayAnimMontage` "/Game/Animation/Mushroom/Mushroom_Alert_Animation_Montage.Mushroom_Alert_Animation_Montage"))

(fn `SetBlackboardIsAttacking`
  (params (IsAttacking :type Boolean))
  (bind _returnvalue (`AIBlueprintHelperLibrary.GetBlackboard` (`AIBlueprintHelperLibrary.GetAIController` self)))
  (`/Engine/EditorBlueprintResources/StandardMacros.IsValid` _returnvalue
    (:`Is Valid`
      (`BlackboardComponent.SetValueAsBool` _returnvalue "Attacking" IsAttacking))))

(fn `SetBlackBoardIsInactive`
  (params (Inactive :type Boolean))
  (`BlackboardComponent.SetValueAsBool` (`AIBlueprintHelperLibrary.GetBlackboard` (`AIBlueprintHelperLibrary.GetAIController` self)) "IsInactive" Inactive))

(fn `SetBlackboardTargetActor`
  (bind _asplayer (cast `/Game/Player` (`GameplayStatics.GetPlayerCharacter` 0)))
  (bind _output_get (set `self.As Player` _asplayer))
  (`BlackboardComponent.SetValueAsObject` (`AIBlueprintHelperLibrary.GetBlackboard` (`AIBlueprintHelperLibrary.GetAIController` self)) "TargetActor" _output_get))

(fn `SetBlackboardTargetVisible`
  (`BlackboardComponent.SetValueAsBool` (`AIBlueprintHelperLibrary.GetBlackboard` (`AIBlueprintHelperLibrary.GetAIController` self)) "TargetVisible" true)
  (return))

(fn `UserConstructionScript`
  (`parent.UserConstructionScript`))