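; Static mushroom NPC that plays a looping idle animation as a non-moving character.
; On BeginPlay it applies a random material from MatArray to the first slot of its skeletal mesh for visual variety.
; Boolean flags for sitting, sitting talking and standing talking then select the looping animation, checked independently in sequence, so the last true flag wins.
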(event `self.ReceiveBeginPlay`
  (bind _output_get (set `self.MAT` (`|GetArrayItem` (`self.MatArray`) (`KismetMathLibrary.RandomIntegerInRange` 0 (- (`KismetArrayLibrary.Array_Length` (`self.MatArray`)) 1)))))
  (`PrimitiveComponent.SetMaterial` (`self.SkeletalMesh`) 0 _output_get)
  (`|ExecutionSequence`
    (:`then_0`
      (if (`self.IsSitting`)
        (`SkeletalMeshComponent.PlayAnimation` (`self.SkeletalMesh`) "/Game/Animation/Mushroom/EvenNew/Mushroom_Sitting_Idle_Animation.Mushroom_Sitting_Idle_Animation" true)))
    (:`then_1`
      (if (`self.IsSittingTalking`)
        (`SkeletalMeshComponent.PlayAnimation` (`self.SkeletalMesh`) "/Game/Animation/Mushroom/EvenNew/Mushroom_Talking_Sitting_Idle_Animation.Mushroom_Talking_Sitting_Idle_Animation" true)))
    (:`then_2`
      (if (`self.IsStandingTalking`)
        (`SkeletalMeshComponent.PlayAnimation` (`self.SkeletalMesh`) "/Game/Animation/Mushroom/EvenNew/Mushroom_Talking_Idle_Animation.Mushroom_Talking_Idle_Animation" true)))))

(fn `UserConstructionScript`)