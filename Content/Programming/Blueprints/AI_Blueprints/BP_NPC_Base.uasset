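; Base NPC character, apparently a mushroom, that can turn and wave at the player.
; On BeginPlay it applies a random body material, stores its rotation and zeroes walk speed when inactive.
; When ShouldWave is set, a player entering WaveCol triggers a timeline turn, a wave montage, then a timeline turn back.
; SetFaceSprite lazily creates a dynamic face material and selects expressions through its Index parameter.
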(event `self.ReceiveBeginPlay`
  (`parent.ReceiveBeginPlay`)
  (if (`self.IsInactive`)
    (set `CharacterMovementComponent.MaxWalkSpeed` 0.0 (`self.CharacterMovement`)))
  (bind _output_get (set `self.MAT` (`|GetArrayItem` (`self.MatArray`) (`KismetMathLibrary.RandomIntegerInRange` 0 (- (`KismetArrayLibrary.Array_Length` (`self.MatArray`)) 1)))))
  (`PrimitiveComponent.SetMaterial` (`self.Mesh`) 0 _output_get)
  (set `self.Starting Rotation` (`self.K2_GetActorRotation`)))

(event `self.WaveCol.OnComponentBeginOverlap`
  (params (OverlappedComponent :type "PrimitiveComponent Object Reference") (OtherActor :type "Actor Object Reference") (OtherComp :type "PrimitiveComponent Object Reference") (OtherBodyIndex :type Integer) (bFromSweep :type Boolean) (SweepResult :type "HitResult Structure (by ref)"))
  (if (and (`self.ActorHasTag` OtherActor "Player") (`self.ShouldWave`))
    (set `self.TargetRotation` (`KismetMathLibrary.FindLookAtRotation` (`self.K2_GetActorLocation`) (`self.K2_GetActorLocation` OtherActor)))
    (bind (_direction _alpha) (`Timeline|RotationLerp` :!via `PlayFromStart`)
      (:`Update`
        (`self.K2_SetActorRotation` (`KismetMathLibrary.RLerp` (`self.Starting Rotation`) (`self.TargetRotation`) _alpha)))
      (:`Finished`
        (bind _returnvalue (`self.PlayAnimMontage` "/Game/Animation/Mushroom/New/Mushroom_Waving_Animation_Montage.Mushroom_Waving_Animation_Montage"))
        (`KismetSystemLibrary.Delay` _returnvalue)
        (bind (_direction_2 _alpha_2) (`Timeline|Timeline` :!via `PlayFromStart`)
          (:`Update`
            (`self.K2_SetActorRotation` (`KismetMathLibrary.RLerp` (`self.TargetRotation`) (`self.Starting Rotation`) _alpha_2))))))))

(fn `SetFaceSprite`
  (params (`Face Index` :type "Float (double-precision)"))
  (`self.CreatedDynamicFace`
    (:`then`
      _)
    (:`else`
      (bind _returnvalue (`PrimitiveComponent.CreateDynamicMaterialInstance` (`self.Mushroom_Face_Varients_Angry_Face`) 0 "/Game/Material/M_MushroomFace_Enemy.M_MushroomFace_Enemy" "None"))
      (set `self.CreatedDynamicFace` _returnvalue)))
  (`MaterialInstanceDynamic.SetScalarParameterValue` (`self.CreatedDynamicFace`) "Index" `Face Index`))

(fn `UserConstructionScript`
  (`parent.UserConstructionScript`))